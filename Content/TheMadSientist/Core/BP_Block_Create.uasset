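; BP_Block_Create is a destructible crate block that loses health when a projectile hits it.
; Each TakeDamage call decrements HealthPoints, and at zero or below the block spawns a Niagara explosion at its location and destroys itself.
; While it survives at or below CrackTreshold, a DoOnce swaps its texture to the cracked crate a single time.
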(event EventBeginPlay
  (|CallParentFunction) ; This node is disabled and will not be called.\nDrag off pins to build functionality.
)

(event Collision|EventActorBeginOverlap
  (params (OtherActor :type Actor%20Object%20Reference))
  (|CallParentFunction OtherActor) ; This node is disabled and will not be called.\nDrag off pins to build functionality.
)

(event EventTick
  (params (DeltaSeconds :type Float%20%28single-precision%29))
  (|CallParentFunction DeltaSeconds) ; This node is disabled and will not be called.\nDrag off pins to build functionality.
)

(event EventTakeDamage
  ;[1 1 1] Gére la prise de dégâts lorsqu'on est touché par un projectille
  (bind _result (Math|Integer|DecrementInt (Variables|Default|GetHealthPoints))
    (:%20%20
      (if (<= _result 0)
        (Niagara|SpawnSystematLocation "/Game/TheMadSientist/Core/NS_Explosion.NS_Explosion" (Transformation|GetActorLocation))
        (Actor|DestroyActor)
        (elif (<= _result (Variables|Default|GetCrackTreshold))
          (Utilities|FlowControl|DoOnce false
            (:Completed
              (CallFunction|UpdateTexture "/Game/TheMadSientist/Art/Interactables/Crate/T_Crate_Cracked.T_Crate_Cracked"))))))))

(fn ConstructionScript
  (|CallParentFunction))