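; Player character for a 2.5D flipbook platformer with walk, jump, crouch, mid-air dive and projectile fire.
; Enhanced Input drives movement along actor forward; diving slams down and notifies BPI_Diveable actors on landing.
; Tick pins camera height, flips the sprite by velocity and selects flipbooks from movement state.
; A timeline rotates the actor 90 degrees for perspective shifts with input disabled, while a DoOnce gates firing until enabled and between cooldowns.
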(event Custom|TriggerCooldown
  ;[1 1 1] Gère le tir de projectile
  (Utilities|FlowControl|Delay 0.2)
  (Utilities|FlowControl|DoOnce true) ; enters at Reset
)

(event Custom|EnableProjectile
  ;[1 1 1] Gère le tir de projectile
  (Utilities|FlowControl|DoOnce true) ; enters at Reset
)

(event Custom|TriggerPerspectiveShifting
  (params (Shift%20Right :type Boolean))
  (bind _returnvalue (Transformation|GetActorRotation))
  ;[1 1 1] Gère la mécanique de shift
  (Variables|Default|SetYawOffset (Math|Float|SelectFloat -9e+01 9e+01 Shift%20Right))
  (Variables|Default|SetInitialYaw (.yaw (Transformation|GetActorRotation)))
  (Input|DisableInput (Game|GetPlayerController 0))
  (Variables|/Script/Engine.MovementComponent|SetVelocity (Variables|Character|GetCharacterMovement) "0, 0, 0")
  (bind _lerpfactor (Timeline|PerspectiveShifting PlayFromStart)
    (:Update
      (Transformation|SetActorRotation (Math|Rotator|MakeRotator (.roll _returnvalue) (.pitch _returnvalue) (+ (* _lerpfactor (Variables|Default|GetYawOffset)) (Variables|Default|GetInitialYaw)))))
    (:Finished
      (Input|EnableInput (Game|GetPlayerController 0)))))

(event Input|EnhancedActionEvents|EnhancedInputActionINP_FireProjectile
  (params (ActionValue :type Boolean) (ElapsedSeconds :type Float%20%28double-precision%29) (TriggeredSeconds :type Float%20%28double-precision%29) (InputAction :type Input%20Action%20Object%20Reference :default "/Game/TheMadSientist/Core/Inputs/INP_FireProjectile.INP_FireProjectile"))
  ;[1 1 1] Gère le tir de projectile
  (:Started
    (Utilities|FlowControl|DoOnce true
      (:Completed
        (Game|SpawnActorfromClass "/Game/TheMadSientist/Core/BP_Projectile.BP_Projectile_C" (Math|Transform|MakeTransform (Transformation|GetActorLocation) (Transformation|GetWorldRotation (Variables|Default|GetSprite)) "1.000000,1.000000,1.000000") "Undefined" "MultiplyWithRoot" 0 0)
        (Audio|SpawnSound2D "/Game/TheMadSientist/Audio/A_Shoot.A_Shoot" 0.5 1.0 0.0 0)
        (CallFunction|TriggerCooldown)))))

(event Input|EnhancedActionEvents|EnhancedInputActionINP_MoveAround
  (params (ActionValue :type Float%20%28double-precision%29) (ElapsedSeconds :type Float%20%28double-precision%29) (TriggeredSeconds :type Float%20%28double-precision%29) (InputAction :type Input%20Action%20Object%20Reference :default "/Game/TheMadSientist/Core/Inputs/INP_MoveAround.INP_MoveAround"))
  ;[1 1 1] Gere les deplacements
  (:Triggered
    (Pawn|Input|AddMovementInput (Transformation|GetActorForwardVector) ActionValue false)))

(event Input|EnhancedActionEvents|EnhancedInputActionINP_Jump
  (params (ActionValue :type Boolean) (ElapsedSeconds :type Float%20%28double-precision%29) (TriggeredSeconds :type Float%20%28double-precision%29) (InputAction :type Input%20Action%20Object%20Reference :default "/Game/TheMadSientist/Core/Inputs/INP_Jump.INP_Jump"))
  (bind _charactermovement (Variables|Character|GetCharacterMovement))
  ;[1 1 1] Gere le saut
  (:Started
    (Character|Jump)
    (if (Math|Boolean|NORBoolean (AI|Components|NavMovement|IsCrouching _charactermovement) (AI|Components|NavMovement|IsFalling _charactermovement))
      (Audio|SpawnSound2D "/Game/TheMadSientist/Audio/A_Jump.A_Jump" 0.3 1.0 0.0 0)))
  (:Completed
    (Character|StopJumping)))

(event Input|EnhancedActionEvents|EnhancedInputActionINP_Crouch
  (params (ActionValue :type Boolean) (ElapsedSeconds :type Float%20%28double-precision%29) (TriggeredSeconds :type Float%20%28double-precision%29) (InputAction :type Input%20Action%20Object%20Reference :default "/Game/TheMadSientist/Core/Inputs/INP_Crouch.INP_Crouch"))
  (bind _sprite (Variables|Default|GetSprite))
  ;[1 1 1] Gere le dive et laccroupissement
  (:Started
    (if (AI|Components|NavMovement|IsFalling (Variables|Character|GetCharacterMovement))
      (if (not (Variables|Default|GetDiving))
        (Variables|Default|SetDiving true)
        (Character|LaunchCharacter "0.000000,0.000000,-1500.000000" true true))
      (else
        (Character|Crouch)
        ;;[1 1 1] Reajuste la position du sprite pour le plaquer au sol
        (Transformation|SetRelativeLocation _sprite "0.000000,0.000000,-37.000000" false true))))
  (:Completed
    (Character|UnCrouch)
    (Transformation|SetRelativeLocation _sprite "0.000000,0.000000,-44.000000" false true)))

(event EventBeginPlay
  ;[1 1 1] Definit la configuration des touches par defaut du jeu
  (Input|AddMappingContext (PlayerController|LocalPlayerSubsystems|GetEnhancedInputLocalPlayerSubsystem (Game|GetPlayerController 0)) "/Game/TheMadSientist/Core/Inputs/IMC_Default.IMC_Default" 0 "(bIgnoreAllPressedKeysUntilRelease=True,bForceImmediately=False)"))

(event EventOnLanded
  (params (Hit :type Hit%20Result%20Structure%20%28by%20ref%29))
  (bind _hitactor (Collision|BreakHitResult Hit))
  ;[1 1 1] Des quon dive sur un objet diveable, on lui demande dactiver sa logique
  (Utilities|FlowControl|Sequence
    (:then_0
      (if (and (Utilities|DoesObjectImplementInterface _hitactor "/Game/TheMadSientist/Core/BPI_Diveable.BPI_Diveable_C") (Variables|Default|GetDiving))
        (Class|BPIDiveable|OnHitbyDive(Message) _hitactor)))
    (:then_1
      (Variables|Default|SetDiving false))))

(event EventTick
  (params (DeltaSeconds :type Float%20%28single-precision%29))
  (bind _sprite (Variables|Default|GetSprite))
  (bind _charactermovement (Variables|Character|GetCharacterMovement))
  (bind _camera (Variables|Default|GetCamera))
  (bind _returnvalue (AI|Components|NavMovement|IsCrouching _charactermovement))
  (bind _returnvalue_2 (Transformation|GetWorldLocation _camera))
  ;[1 1 1] Force la hauteur de la caméra
  (Transformation|SetWorldLocation _camera (Math|Vector|MakeVector (.x _returnvalue_2) (.y _returnvalue_2) 4e+02) false false)
  (Utilities|FlowControl|Sequence
    (:then_0
      ;[1 1 1] Orient le sprite en fonction de la direction de marche
      (Math|Float|CompareFloat (Math|Vector|DotProduct (Math|Vector|Normalize (Transformation|GetVelocity)) (Transformation|GetActorForwardVector)) 0.0
        (:>
          (Transformation|SetRelativeRotation _sprite "0, 0, 0" false false))
        (:<
          (Transformation|SetRelativeRotation _sprite "0.000000,180.000000,0.000000" false false))))
    (:then_1
      ;[1 1 1] Gere les animation aeriennes
      (if (AI|Components|NavMovement|IsFalling (Variables|Character|GetCharacterMovement))
        (Sprite|SetFlipbook (Variables|Default|GetSprite) (select (Variables|Default|GetDiving) "/Game/TheMadSientist/Art/Character/PFB_Dive.PFB_Dive" "/Game/TheMadSientist/Art/Character/PFB_Jump.PFB_Jump"))
        (else
          ;[1 1 1] Gere les animation de deplacement au sol
          (if (> (Class|KismetMathLibrary|VSizeXYSquared (Pawn|Components|CharacterMovement|GetCurrentAcceleration (Variables|Character|GetCharacterMovement))) 0.0)
            (Sprite|SetFlipbook (Variables|Default|GetSprite) (select _returnvalue "/Game/TheMadSientist/Art/Character/PFB_CrouchWalk.PFB_CrouchWalk" "/Game/TheMadSientist/Art/Character/PFB_Walk.PFB_Walk"))
            (else
              (Sprite|SetFlipbook (Variables|Default|GetSprite) (select _returnvalue "/Game/TheMadSientist/Art/Character/PFB_CrouchIdle.PFB_CrouchIdle" "/Game/TheMadSientist/Art/Character/PFB_Idle.PFB_Idle")))))))))

(fn ConstructionScript)